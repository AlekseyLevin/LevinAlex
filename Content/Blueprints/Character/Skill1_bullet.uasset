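; Skill 1 bullet actor that turns into an AI-controlled pawn where it hits.
; When its Sphere component registers a hit, it spawns an AI of PawnClass slightly above the bullet, ignoring spawn collision failure.
; The pawn's facing keeps only the X part of the bullet's forward vector, snapping it along the world X axis.
; It then plays a 2D teleport sound and destroys itself.
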(event `self.Sphere.OnComponentHit`
  (params (HitComponent :type "PrimitiveComponent Object Reference") (OtherActor :type "Actor Object Reference") (OtherComp :type "PrimitiveComponent Object Reference") (NormalImpulse :type "Vector Structure") (Hit :type "HitResult Structure (by ref)"))
  (`AIBlueprintHelperLibrary.SpawnAIFromClass` (`self.Pawn Class`) null (+ (.location (`self.GetTransform`)) (0.0 0.0 150.0)) (`KismetMathLibrary.Conv_VectorToRotator` (`KismetMathLibrary.Normal` (* (`self.GetActorForwardVector`) (1.0 0.0 0.0)))) true null)
  (`GameplayStatics.SpawnSound2D` "/Engine/VREditor/Sounds/UI/Teleport_Committed.Teleport_Committed" 1.0 1.0 0.0 null)
  (`self.K2_DestroyActor`))

(fn `UserConstructionScript`)