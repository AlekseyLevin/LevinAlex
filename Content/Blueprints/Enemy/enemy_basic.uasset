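; Basic 2D Paper2D enemy that detects a nearby pawn, steps horizontally toward it, and fires bullets when within attack range.
; Tick runs a timer-gated Status machine (decide, walk, telegraph, shoot), with delays partly taken from flipbook lengths.
; Steps require a trace hit or Suicidal, and animations switch on last frames.
; Damage tints it red with invulnerability until the color restores; death animation precedes destruction.
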(event `self.ReceiveBeginPlay`
  (bind _paperflipbook (`self.PaperFlipbook`))
  (bind _paperflipbook_2 (`self.PaperFlipbook`))
  (bind _output_get (set `self.cloc` (`self.K2_GetActorLocation`)))
  (bind _output_get_2 (set `self.targ` _output_get))
  (set `self.start` _output_get_2)
  (set `self.status` 0)
  (`PaperFlipbookComponent.SetFlipbook` _paperflipbook_2 (`self.telegraph_anim`))
  (set `self.telegraph_length` (`PaperFlipbookComponent.GetFlipbookLength` _paperflipbook_2))
  (`PaperFlipbookComponent.SetFlipbook` _paperflipbook (`self.attack_anim`))
  (set `self.att_reload` (`PaperFlipbookComponent.GetFlipbookLength` _paperflipbook))
  (`PaperFlipbookComponent.SetFlipbook` (`self.PaperFlipbook`) (`self.stand_anim`)))

(event `self.ReceiveTick`
  (params (DeltaSeconds :type "Float (single-precision)"))
  (bind _paperflipbook (`self.PaperFlipbook`))
  (bind _paperflipbook_2 (`self.PaperFlipbook`))
  (bind _static_reload (`self.static_reload`))
  (bind _paperflipbook_3 (`self.PaperFlipbook`))
  (set `self.dt` DeltaSeconds)
  (set `self.cloc` (`self.K2_GetActorLocation`))
  (`|ExecutionSequence`
    (:`then_0`
      (if (`KismetSystemLibrary.IsValid` (`self.Target`))
        (set `self.dir_x` (`self.getdirtoplayer`))))
    (:`then_1`
      (if (and (> (`self.hp`) 0.0) (<= (`self.timer`) 0.0))
        (switch `int` (`self.status`)
          (:`0`
            (set `self.start` (`self.cloc`))
            (if (`KismetSystemLibrary.IsValid` (`self.Target`))
              (if (< (`self.getdisttoplayer`) (`self.att_dst`))
                (set `self.status` 3)
                (set `self.timer` _static_reload)
                (else
                  (set `self.status` 2)
                  (set `self.timer` _static_reload)))
              (set `self.laststat` 0)))
          (:`1`
            (`|SpawnActorFromClass` (`self.bullet`) (`SceneComponent.K2_GetComponentToWorld` (`self.Arrow`)) "AlwaysSpawn" "OverrideRootScale" self null)
            (set `self.timer` (`self.att_reload`))
            (set `self.laststat` 1)
            (set `self.status` 0))
          (:`2`
            (`self.trytowalk` (`self.dir_x`) (`self.t_dist`))
            (set `self.timer` (`self.walk_reload`))
            (set `self.laststat` 2)
            (set `self.status` 0))
          (:`3`
            (set `self.status` 1)
            (set `self.timer` (`self.telegraph_length`))
            (set `self.laststat` 3)
            (`KismetSystemLibrary.PrintString` "to_telegraph")))))
    (:`then_2`
      (if (and (!= (`self.targ`) (`self.cloc`) :`ErrorTolerance` (* (`self.spd`) (`self.dt`) 1.0)) (> (`self.timer`) 0.0))
        (bind _n_loc (`/Game/Blueprints/Main/funclib.movement` (`self.targ`) (`self.start`) (`self.cloc`) (`self.spd`) (`self.dt`)))
        (bind _output_get (set `self.cloc` _n_loc))
        (`self.K2_SetActorLocation` _output_get)))
    (:`then_3`
      (`|ExecutionSequence`
        (:`then_0`
          (if (and (!= (`self.cloc`) (`self.targ`) :`ErrorTolerance` (* (`self.spd`) (`self.dt`) 0.51)) (> (`self.hp`) 0.0))
            (set `self.ftu` (`self.walk_anim`))))
        (:`then_1`
          (if (> (`self.hp`) 0.0)
            (switch `int` (`self.laststat`)
              (:`0`
                (set `self.ftu` (`self.stand_anim`)))
              (:`1`
                (set `self.ftu` (`self.attack_anim`)))
              (:`2`
                _)
              (:`3`
                (set `self.ftu` (`self.telegraph_anim`))))
            (set `self.laststat` 3)
            (elif (!= (`PaperFlipbookComponent.GetFlipbook` (`self.PaperFlipbook`)) (`self.death_anim`))
              (set `self.ftu` (`self.death_anim`))
              (elif (== (`PaperFlipbookComponent.GetPlaybackPositionInFrames` _paperflipbook_2) (- (`PaperFlipbookComponent.GetFlipbookLengthInFrames` _paperflipbook_2) 1))
                (`self.K2_DestroyActor`)))))))
    (:`then_4`
      (if (`KismetSystemLibrary.IsValid` (`self.PaperFlipbook`))
        (if (>= (`self.dir_x`) 0.0)
          (`SceneComponent.K2_SetWorldRotation` _paperflipbook_3 (`KismetMathLibrary.MakeRotator` 0.0 0.0 180.0) false false)
          (else
            (`SceneComponent.K2_SetWorldRotation` _paperflipbook_3 (`KismetMathLibrary.MakeRotator` 0.0) false false)))))
    (:`then_5`
      (if (> (`self.timer`) 0.0)
        (set `self.timer` (- (`self.timer`) (`self.dt`)))))
    (:`then_6`
      (if (`KismetSystemLibrary.IsValid` (`self.PaperFlipbook`))
        (if (and (!= (`PaperFlipbookComponent.GetFlipbook` (`self.PaperFlipbook`)) (`self.ftu`)) (== (`PaperFlipbookComponent.GetPlaybackPositionInFrames` _paperflipbook) (- (`PaperFlipbookComponent.GetFlipbookLengthInFrames` _paperflipbook) 1)))
          (`PaperFlipbookComponent.SetFlipbook` (`self.PaperFlipbook`) (`self.ftu`)))))
    (:`then_7`
      (if (`KismetSystemLibrary.IsValid` (`self.Arrow1`))
        (`SceneComponent.K2_SetWorldLocation` (`self.Arrow1`) (`self.targ`) false false)
        (`self.color_restore`)))
    (:`then_8`
      (`self.Detect`))))

(event `self.ReceiveAnyDamage`
  (params (Damage :type "Float (single-precision)") (DamageType :type "DamageType Object Reference") (InstigatedBy :type "Controller Object Reference") (DamageCauser :type "Actor Object Reference"))
  (if (and (not (`self.invuln`)) (> (`self.hp`) 0.0))
    (set `self.hp` (- (`self.hp`) Damage))
    (`PaperFlipbookComponent.SetSpriteColor` (`self.PaperFlipbook`) (make `LinearColor` 1.0 0.0 0.0 1.0))))

(fn `color_restore`
  (bind _returnvalue (* (`self.dt`) 1.0))
  (bind _spritecolor (`PaperFlipbookComponent.SpriteColor` (`self.PaperFlipbook`)))
  (bind (_r _g _b _a) (break `LinearColor` _spritecolor))
  (if (< (`.B` (break `LinearColor` _spritecolor)) 1.0)
    (set `self.invuln` true)
    (`PaperFlipbookComponent.SetSpriteColor` (`self.PaperFlipbook`) (make `LinearColor` _r (+ _g _returnvalue) (+ _returnvalue _b) _a))
    (else
      (set `self.invuln` false))))

(fn `Detect`
  (`|ExecutionSequence`
    (:`then_0`
      (bind _outactors (`KismetSystemLibrary.SphereOverlapActors` (`self.K2_GetActorLocation`) 400.0 (`|MakeArray` "ObjectTypeQuery3" :!type "EObjectTypeQuery Enum")))
      (if (> (`KismetArrayLibrary.Array_Length` _outactors) 0)
        (set `self.Target` (`|GetArrayItem` _outactors))
        (else
          (set `self.Target` null))))
    (:`then_1`
      (`KismetSystemLibrary.PrintString` (`KismetSystemLibrary.GetDisplayName` (`self.Target`)) true true (struct :`G` 0.66 :`B` 1.0 :`A` 1.0) 0.0))))

(fn `getdirtoplayer`
  (returns (x_k :type "Float (double-precision)"))
  (if (>= (.x (- (`self.K2_GetActorLocation`) (`self.K2_GetActorLocation` (`self.Target`)))) 0.0)
    (return 1.0)
    (else
      (return -1.0))))

(fn `getdisttoplayer`
  (returns (dist :type "Float (double-precision)"))
  (return (`KismetMathLibrary.VSize` (- (`self.K2_GetActorLocation` (`self.Target`)) (`self.K2_GetActorLocation`)))))

(fn `trytowalk`
  (params (kx :type "Float (double-precision)") (td :type "Float (double-precision)"))
  (locals (kxl :type "Float (double-precision)" :default 0.0) (tdl :type "Float (double-precision)" :default 0.0))
  (bind _returnvalue (`KismetMathLibrary.MakeVector` (+ (* (`local.kxl`) (`local.tdl`) -1.0) (.x (`self.K2_GetActorLocation`))) (.y (`self.K2_GetActorLocation`)) (.z (`self.K2_GetActorLocation`))))
  (set `local.kxl` kx)
  (set `local.tdl` td)
  (bind (_outhit _returnvalue_2) (`KismetSystemLibrary.LineTraceSingle` _returnvalue (0.0 0.0 0.0) "TraceTypeQuery1"))
  (if (or _returnvalue_2 (`self.suicidal`))
    (set `self.targ` _returnvalue)
    (set `self.start` (`self.cloc`))))

(fn `UserConstructionScript`)