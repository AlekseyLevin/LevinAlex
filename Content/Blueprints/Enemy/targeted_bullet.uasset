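; Enemy projectile that is aimed at the player's location captured when it spawns, so it does not home.
; Each tick counts down its lifetime and moves it via a Movement helper fed by origin, target, current position and speed.
; A distance check against the live player position applies Dmg and destroys it.
; Separately, sphere overlap with any non-owner applies Damage, switches the flipbook to Fireball1 and destroys it after a brief delay.
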(event `self.ReceiveBeginPlay`
  (set `self.target` (`self.K2_GetActorLocation` (`GameplayStatics.GetPlayerPawn` 0)))
  (bind _output_get (set `self.origin` (`self.K2_GetActorLocation`)))
  (set `self.cloc` _output_get))

(event `self.ReceiveTick`
  (params (DeltaSeconds :type "Float (single-precision)"))
  (bind _output_get (set `self.dt` DeltaSeconds))
  (set `self.life` (- (`self.life`) _output_get))
  (if (> (`self.life`) 0.0)
    (bind _n_loc (`/Game/Blueprints/Main/funclib.movement` (`self.target`) (`self.origin`) (`self.cloc`) (`self.spd`) (`self.dt`)))
    (bind _output_get_2 (set `self.cloc` _n_loc))
    (`self.K2_SetActorLocation` _output_get_2)
    (bind _d (`/Game/Blueprints/Main/funclib.getdist` (`self.K2_GetActorLocation` (`GameplayStatics.GetPlayerPawn` 0)) (`self.cloc`)))
    (if (< _d 15.0)
      (`GameplayStatics.ApplyDamage` (`GameplayStatics.GetPlayerPawn` 0) (`self.dmg`))
      (`self.K2_DestroyActor`))
    (else
      (`self.K2_DestroyActor`))))

(event `self.Sphere.OnComponentBeginOverlap`
  (params (OverlappedComponent :type "PrimitiveComponent Object Reference") (OtherActor :type "Actor Object Reference") (OtherComp :type "PrimitiveComponent Object Reference") (OtherBodyIndex :type Integer) (bFromSweep :type Boolean) (SweepResult :type "HitResult Structure (by ref)"))
  (if (!= OtherActor (`self.GetOwner`))
    (`GameplayStatics.ApplyDamage` OtherActor (`self.Damage`))
    (`PaperFlipbookComponent.SetFlipbook` (`self.PaperFlipbook`) "/Game/2DSideScroller/2DGraveyardPackHandcraftedArt/Sprites/fireball1.fireball1")
    (`KismetSystemLibrary.Delay` 0.2)
    (`self.K2_DestroyActor`)))

(fn `UserConstructionScript`)