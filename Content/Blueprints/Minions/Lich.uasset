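; Lich minion Blueprint that walks in a straight line, flags itself to shoot and removes itself after a short lifetime.
; BeginPlay stores a movement direction from the normalized X component of its forward vector, locking travel to the world X axis.
; Each Tick applies that movement and sets Needshoot, which nothing here reads, while a Delay started from Tick destroys the actor about two seconds later.
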(event `self.ReceiveBeginPlay`
  (`parent.ReceiveBeginPlay`)
  (set `self.Initial_Direction` (`KismetMathLibrary.Normal` (* (`self.GetActorForwardVector`) (1.0 0.0 0.0)))))

(event `self.ReceiveTick`
  (params (DeltaSeconds :type "Float (single-precision)"))
  (`parent.ReceiveTick` DeltaSeconds)
  (`self.AddMovementInput` (`self.Initial_Direction`))
  (set `self.needshoot` true)
  (`KismetSystemLibrary.Delay` 2.0)
  (`self.K2_DestroyActor`))

(fn `UserConstructionScript`
  (`parent.UserConstructionScript`))