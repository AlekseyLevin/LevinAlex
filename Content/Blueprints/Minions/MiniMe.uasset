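; MiniMe is a short-lived minion pawn that walks in a straight line, spawns MiniZombie AI pawns, then destroys itself.
; BeginPlay locks the movement direction to the world X component of its forward vector.
; Latent Delays on Tick re-arm, so spawns with a teleport sound repeat about every 1.5 seconds until destruction, 3 seconds after the first.
; CHECKDEATH is empty, and a duplicate spawn-and-destroy chain is unconnected.
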(event `self.ReceiveBeginPlay`
  (`parent.ReceiveBeginPlay`)
  (set `self.Initial_Direction` (`KismetMathLibrary.Normal` (* (`self.GetActorForwardVector`) (1.0 0.0 0.0)))))

(event `self.ReceiveTick`
  (params (DeltaSeconds :type "Float (single-precision)"))
  (`parent.ReceiveTick` DeltaSeconds)
  (`self.AddMovementInput` (`self.Initial_Direction`))
  (`KismetSystemLibrary.Delay` 1.5)
  (`AIBlueprintHelperLibrary.SpawnAIFromClass` "/Game/Blueprints/Minions/MiniZombie.MiniZombie_C" null (+ (.location (`self.GetTransform`)) (40.0 0.0 10.0)) (`KismetMathLibrary.Conv_VectorToRotator` (`KismetMathLibrary.Normal` (* (`self.GetActorForwardVector`) (1.0 0.0 0.0)))) true null)
  (`GameplayStatics.SpawnSound2D` "/Engine/VREditor/Sounds/UI/Teleport_Committed.Teleport_Committed" 1.0 1.0 0.0 null)
  (`KismetSystemLibrary.Delay` 3.0)
  (`self.K2_DestroyActor`))

(event `self.CHECK_DEATH`)

(fn `UserConstructionScript`
  (`parent.UserConstructionScript`))