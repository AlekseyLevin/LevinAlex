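; Vampire is a minion Blueprint that walks in a fixed direction and heals itself when it deals damage.
; BeginPlay stores its forward vector, flattened to the X axis and normalized, and Tick feeds that into movement input while setting WannaHit every frame.
; Its CustomApplyDamage override runs the parent logic, then adds one HP, clamped between zero and MaxHP.
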(event `self.ReceiveBeginPlay`
  (`parent.ReceiveBeginPlay`)
  (set `self.Initial_Direction` (`KismetMathLibrary.Normal` (* (`self.GetActorForwardVector`) (1.0 0.0 0.0)))))

(event `self.ReceiveTick`
  (params (DeltaSeconds :type "Float (single-precision)"))
  (`parent.ReceiveTick` DeltaSeconds)
  (`self.AddMovementInput` (`self.Initial_Direction`))
  (set `self.wanna_hit` true))

(event `self.CustomApplyDamage`
  (params (DamagedActor :type "Actor Object Reference"))
  (`parent.CustomApplyDamage` DamagedActor)
  (set `self.HP current` (`KismetMathLibrary.FClamp` (+ (`self.HP current`) 1.0) 0.0 (`self.Max HP`))))

(fn `UserConstructionScript`
  (`parent.UserConstructionScript`))