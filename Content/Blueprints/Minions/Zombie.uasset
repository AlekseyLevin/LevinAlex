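; Zombie is a short-lived minion Blueprint that walks in a straight line, then leaves a Tomb behind.
; On BeginPlay it locks its direction to the normalized world X component of its forward vector.
; Tick applies that movement input and keeps WannaHit set.
; A Delay inside Tick serves as its lifetime timer, after which it spawns the Tomb at a slight X offset and destroys itself.
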(event `self.ReceiveBeginPlay`
  (`parent.ReceiveBeginPlay`)
  (set `self.Initial_Direction` (`KismetMathLibrary.Normal` (* (`self.GetActorForwardVector`) (1.0 0.0 0.0)))))

(event `self.ReceiveTick`
  (params (DeltaSeconds :type "Float (single-precision)"))
  (`parent.ReceiveTick` DeltaSeconds)
  (`self.AddMovementInput` (`self.Initial_Direction`))
  (set `self.wanna_hit` true)
  (`KismetSystemLibrary.Delay` 3.0)
  (`|SpawnActorFromClass` "/Game/Blueprints/Minions/Tomb.Tomb_C" (`KismetMathLibrary.Conv_VectorToTransform` (+ (.location (`self.GetTransform`)) (-5.0 0.0 0.0))) "AlwaysSpawn" "OverrideRootScale" null null)
  (`self.K2_DestroyActor`))

(fn `UserConstructionScript`
  (`parent.UserConstructionScript`))