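; Bomb actor for the lich minion that explodes when its Sphere component registers a hit.
; On hit, it gathers all Pawns in a fixed radius and applies point damage to each, directed outward from the bomb, with no falloff or team filtering.
; It then plays a non-spatialized 2D sound and destroys itself.
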(event `self.Sphere.OnComponentHit`
  (params (HitComponent :type "PrimitiveComponent Object Reference") (OtherActor :type "Actor Object Reference") (OtherComp :type "PrimitiveComponent Object Reference") (NormalImpulse :type "Vector Structure") (Hit :type "HitResult Structure (by ref)"))
  (set `self.Other Actor` OtherActor)
  (set `self.Hit Info` Hit)
  (bind _outactors (`KismetSystemLibrary.SphereOverlapActors` (`self.K2_GetActorLocation`) 200.0 (`|MakeArray` "ObjectTypeQuery3" :!type "EObjectTypeQuery Enum")))
  (set `self.TargetsArray` _outactors)
  (for _array_element (`self.TargetsArray`)
    (`GameplayStatics.ApplyPointDamage` _array_element (`self.Base Damage`) (`KismetMathLibrary.Normal` (- (`self.K2_GetActorLocation` _array_element) (`self.K2_GetActorLocation`))) (`self.Hit Info`) null self))
  (`GameplayStatics.SpawnSound2D` "/Engine/VREditor/Sounds/UI/Teleport_Mode_Entered.Teleport_Mode_Entered" 1.0 1.0 0.0 null)
  (`self.K2_DestroyActor`))

(fn `UserConstructionScript`)