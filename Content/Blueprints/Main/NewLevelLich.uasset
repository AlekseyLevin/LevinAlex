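; NewLevelLich is an overlap trigger that grants a skill and records level progress for the player's side-scroller character.
; When a player-controlled 2DSideScrollerCharacter enters its Box, it passes NewSkill to AddSkills on the character's Gi reference and then sets CurrentLevel there.
; An OpenLevelByName node for LevelName is present but unconnected, so the trigger does not change levels itself.
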(event `self.Box.OnComponentBeginOverlap`
  (params (OverlappedComponent :type "PrimitiveComponent Object Reference") (OtherActor :type "Actor Object Reference") (OtherComp :type "PrimitiveComponent Object Reference") (OtherBodyIndex :type Integer) (bFromSweep :type Boolean) (SweepResult :type "HitResult Structure (by ref)"))
  (bind _as2dside_scroller_character (cast `/Game/Blueprints/Character/2DSideScrollerCharacter` OtherActor))
  (if (`Pawn.IsPlayerControlled` _as2dside_scroller_character)
    (`/Game/Blueprints/Main/MainGameInstance.AddSkills` (`/Game/Blueprints/Character/2DSideScrollerCharacter.gi` _as2dside_scroller_character) (`self.New Skill`))
    (set `/Game/Blueprints/Main/MainGameInstance.CurrentLevel` (`self.Current Level`) (`/Game/Blueprints/Character/2DSideScrollerCharacter.gi` _as2dside_scroller_character))))

(fn `UserConstructionScript`)