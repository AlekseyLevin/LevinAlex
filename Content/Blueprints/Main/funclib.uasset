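; Blueprint function library with shared math helpers for linear movement and distance.
; Movement advances a current location by speed times delta time along the start-to-end direction, changing only X and Z and leaving Y untouched.
; The direction is divided by the full 3D length, with no zero-length guard or clamp at the end point.
; Getdist returns the straight-line distance between two vectors.
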(fn `getdist`
  (params (a :type "Vector Structure") (b :type "Vector Structure"))
  (returns (d :type "Float (double-precision)"))
  (return (`KismetMathLibrary.VSize` (- a b))))

(fn `movement`
  (params (e_loc :type "Vector Structure") (s_loc :type "Vector Structure") (c_loc :type "Vector Structure") (spd :type "Float (double-precision)") (dt :type "Float (double-precision)"))
  (returns (n_loc :type "Vector Structure"))
  (locals (kx :type "Float (double-precision)") (kz :type "Float (double-precision)") (d :type "Float (double-precision)") (cloc_add :type "Vector Structure") (dt_loc :type "Float (double-precision)") (spd_loc :type "Float (double-precision)"))
  (bind _returnvalue (- e_loc s_loc))
  (bind _returnvalue_2 (`KismetMathLibrary.VSize` _returnvalue))
  (bind _returnvalue_3 (* (`local.dt_loc`) (`local.spd_loc`)))
  (set `local.dt_loc` dt)
  (set `local.spd_loc` spd)
  (set `local.cloc_add` c_loc)
  (`|ExecutionSequence`
    (:`then_0`
      (set `local.kx` (/ (.x _returnvalue) _returnvalue_2))
      (set `local.kz` (/ (.z _returnvalue) _returnvalue_2)))
    (:`then_1`
      (bind _output_get (set `local.cloc_add` (`KismetMathLibrary.MakeVector` (+ (.x (`local.cloc_add`)) (* _returnvalue_3 (`local.kx`))) (.y (`local.cloc_add`)) (+ (.z (`local.cloc_add`)) (* _returnvalue_3 (`local.kz`))))))
      (return _output_get))))