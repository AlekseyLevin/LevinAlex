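; Game instance that manages menu display, new game start and some player state such as HP percentage and available skills.
; Menu events lazily create and cache the main and options widgets, with the main menu switching to cursor-driven UI-only input.
; New game restores game-only input and opens Level001, while a level-loaded event sets the current level from an alias map lookup.
; Helper functions compute the HP ratio and add unique skills.
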(event `ShowMainMenu`
  (bind _returnvalue (`GameplayStatics.GetPlayerController` 0))
  ;[1 1 1] Main Menu
  (`/Engine/EditorBlueprintResources/StandardMacros.IsValid` (`self.MainMenu`)
    (:`Is Valid`
      _)
    (:`Is Not Valid`
      (bind _returnvalue_2 (`|CreateWidget` "/Game/Blueprints/UI/MainMenu.MainMenu_C" _returnvalue))
      (set `self.MainMenu` _returnvalue_2)))
  (`UserWidget.AddToViewport` (`self.MainMenu`) 0)
  (set `PlayerController.bShowMouseCursor` true _returnvalue)
  (`WidgetBlueprintLibrary.SetInputMode_UIOnlyEx` _returnvalue (`self.MainMenu`) "LockInFullscreen"))

(event `ShowOptionsMenu`
  ;[1 1 1] Options Menu
  (`/Engine/EditorBlueprintResources/StandardMacros.IsValid` (`self.OptionsMenu`)
    (:`Is Valid`
      _)
    (:`Is Not Valid`
      (bind _returnvalue (`|CreateWidget` "/Game/Blueprints/UI/OptionsMenu.OptionsMenu_C" (`GameplayStatics.GetPlayerController` 0)))
      (set `self.OptionsMenu` _returnvalue)))
  (`UserWidget.AddToViewport` (`self.OptionsMenu`) 0))

(event `Create New Game`
  ;[1 1 1] New Game
  (`WidgetBlueprintLibrary.SetInputMode_GameOnly` (`GameplayStatics.GetPlayerController` 0))
  (`GameplayStatics.OpenLevel` "Level001"))

(event `NewLevelLoaded`
  (params (Key :type Name))
  (set `self.CurrentLevel` (`BlueprintMapLibrary.Map_Find` (`self.LevelAllias`) Key)))

(fn `AddSkills`
  (params (NewSkill :type "/Game/Blueprints/Character/E_Skills Enum" :default "NewEnumerator0"))
  (`KismetArrayLibrary.Array_AddUnique` (`self.AvailableSkills`) NewSkill))

(fn `calchpperc`
  (set `self.hpperc` (/ (`KismetMathLibrary.Conv_IntToDouble` (`self.hp`)) (`KismetMathLibrary.Conv_IntToDouble` (`self.maxhp`)))))